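; First-person vampire player character for a networked game, handling HUD, proximity voice chat, ability feedback and death.
; BeginPlay registers a spatialized VOIP talker, retrying until PlayerState is valid, and creates the HUD widgets.
; Ability, item, dialog and shop component events drive widgets, sounds and effects through client events, while health and damage tint refresh every Tick.
; On death, a server event possesses a spawned spectator and destroys the pawn.
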(event `Key|Escape`
  (params (Key :type "Key Structure"))
  (:`Pressed`
    (`KismetSystemLibrary.QuitGame` null "Quit")))

(event `Key|N`
  (params (Key :type "Key Structure"))
  (:`Pressed`
    (`KismetSystemLibrary.ExecuteConsoleCommand` "stat net" null)))

(event `Key|V`
  (params (Key :type "Key Structure"))
  (:`Pressed`
    (bind _asplayer_controller (cast `PlayerController` (`self.GetController` self)))
    (`/Engine/EditorBlueprintResources/StandardMacros.FlipFlop`
      (:`A`
        (`KismetSystemLibrary.ExecuteConsoleCommand` "ToggleSpeaking 0" _asplayer_controller) ; Turn Off VC
      )
      (:`B`
        (`KismetSystemLibrary.ExecuteConsoleCommand` "ToggleSpeaking 1" _asplayer_controller) ; Turn On VC
      ))))

(event `self.ReceiveBeginPlay`
  (bind _returnvalue (`KismetMathLibrary.RandomInteger` 1000000))
  (bind _playerstate (`self.PlayerState`))
  (bind _widgetinteraction (`self.WidgetInteraction`))
  (`|ExecutionSequence`
    (:`then_0`
      (bind _returnvalue_2 (`AddComponent|NODE_AddVOIPTalker-2`))
      (bind _output_get (set `self.VOIPTalker` _returnvalue_2))
      (`/Engine/EditorBlueprintResources/StandardMacros.IsValid` _playerstate :!label _label
        (:`Is Valid`
          (`VOIPTalker.RegisterWithPlayerState` _output_get _playerstate)
          (`VOIPStatics.SetMicThreshold` -5.0)
          (set `VOIPTalker.Settings` (make `VoiceSettings` (`self.FirstPersonCameraComponent`) "/Game/Frazier/Creative/Player/VC_SoundAttenuation.VC_SoundAttenuation" "/Game/Frazier/Creative/Player/VC_EffectChain.VC_EffectChain") (`self.VOIPTalker`))
          (`AdvancedVoiceLibrary.RegisterRemoteTalker` (`AdvancedSessionsLibrary.GetUniqueNetIDFromPlayerState` _playerstate))
          (bind _asbp_first_person_player_controller (cast `/Game/FirstPerson/Blueprints/BP_FirstPersonPlayerController` (`self.GetController` self)))
          (`KismetSystemLibrary.ExecuteConsoleCommand` "ToggleSpeaking 1" _asbp_first_person_player_controller) ; Turn On VC
        )
        (:`Is Not Valid`
          (`KismetSystemLibrary.Delay` 1.0)
          (goto _label))))
    (:`then_1`
      (bind _asplayer_controller (cast `PlayerController` (`self.GetController` self)))
      (`|ExecutionSequence`
        (:`then_0`
          (bind _returnvalue_3 (`|CreateWidget` "/Game/Frazier/Creative/Player/WBP_AbilityDisplay.WBP_AbilityDisplay_C" _asplayer_controller))
          (bind _output_get_2 (set `self.AbilityDisplay` _returnvalue_3))
          (`UserWidget.AddToViewport` _output_get_2 0))
        (:`then_1`
          (bind _returnvalue_4 (`|CreateWidget` "/Game/Frazier/Creative/Player/WBP_Health.WBP_Health_C" _asplayer_controller))
          (bind _output_get_3 (set `self.HealthDisplay` _returnvalue_4))
          (`UserWidget.AddToViewport` _output_get_3 0)
          (`self.ClientUpdateHealthDisplay`))
        (:`then_2`
          (bind _returnvalue_5 (`|CreateWidget` "/Game/Frazier/Creative/Items/WBP_ItemDisplay.WBP_ItemDisplay_C" _asplayer_controller))
          (bind _output_get_4 (set `self.ItemDisplay` _returnvalue_5))
          (`UserWidget.AddToViewport` _output_get_4 0)
          (`self.ClientUpdateItemDisplay`))
        (:`then_3`
          (bind _returnvalue_6 (`|CreateWidget` "/Game/Frazier/Creative/Lair/WBP_Dialog.WBP_Dialog_C" _asplayer_controller))
          (bind _output_get_5 (set `self.DialogDisplay` _returnvalue_6))
          (`UserWidget.AddToViewport` _output_get_5 0)
          (`Widget.SetVisibility` _output_get_5 "Collapsed"))
        (:`then_4`
          (bind _returnvalue_7 (`|CreateWidget` "/Game/Frazier/Creative/Lair/WBP_Shop.WBP_Shop_C" _asplayer_controller))
          (bind _output_get_6 (set `self.ShopDisplay` _returnvalue_7))
          (`UserWidget.AddToViewport` _output_get_6 0)
          (`Widget.SetVisibility` _output_get_6 "Collapsed"))
        (:`then_5`
          (bind _returnvalue_8 (`|CreateWidget` "/Game/Frazier/Creative/WBP_Damaged.WBP_Damaged_C" _asplayer_controller))
          (bind _output_get_7 (set `self.DamageTintDisplay` _returnvalue_8))
          (`UserWidget.AddToViewport` _output_get_7 0))))
    (:`then_2`
      (set `WidgetInteractionComponent.PointerIndex` _returnvalue _widgetinteraction)
      (set `WidgetInteractionComponent.VirtualUserIndex` _returnvalue _widgetinteraction))))

(event `self.ReceiveTick`
  (params (DeltaSeconds :type "Float (single-precision)"))
  (`self.ClientUpdateHealthDisplay`))

(event `ClientUpdateHealthDisplay`
  (bind _combat (`self.Combat`))
  (bind _combat_2 (`self.Combat`))
  (bind _damagetintdisplay (`self.DamageTintDisplay`))
  (bind _healthdisplay (`self.HealthDisplay`))
  (`|ExecutionSequence`
    (:`then_0`
      (`/Engine/EditorBlueprintResources/StandardMacros.IsValid` _healthdisplay
        (:`Is Valid`
          (`/Engine/EditorBlueprintResources/StandardMacros.IsValid` _combat_2
            (:`Is Valid`
              (set `/Game/Frazier/Creative/Player/WBP_Health.HealthPercent` (`KismetMathLibrary.MapRangeClamped` (`CombatComponent.Health` _combat_2) 0.0 (`CombatComponent.MaxHealth` _combat_2) 0.0 1.0) _healthdisplay))))))
    (:`then_1`
      (`/Engine/EditorBlueprintResources/StandardMacros.IsValid` _damagetintdisplay
        (:`Is Valid`
          (`/Engine/EditorBlueprintResources/StandardMacros.IsValid` _combat
            (:`Is Valid`
              (set `/Game/Frazier/Creative/WBP_Damaged.Tint` (make `SlateColor` (make `LinearColor` 0.360784 0.035294 0.043137 (`KismetMathLibrary.MapRangeClamped` (`CombatComponent.Health` _combat) 0.0 (`CombatComponent.MaxHealth` _combat) 0.5 -0.3))) _damagetintdisplay))))))))

(event `self.VampireAttack.OnBiteCooldownBegin`
  (params (BiteCooldown :type "Float (single-precision)"))
  (bind _abilitydisplay (`self.AbilityDisplay`))
  (bind _bite (`/Game/Frazier/Creative/Player/WBP_AbilityDisplay.Bite` _abilitydisplay))
  (`/Engine/EditorBlueprintResources/StandardMacros.IsValid` _abilitydisplay
    (:`Is Valid`
      (`UserWidget.PlayAnimation` _bite (`/Game/Frazier/Creative/Player/WBP_BiteAbilityUI.Cooldown` _bite) 0.0 1 "Forward" (/ 1.0 BiteCooldown) true))))

(event `self.VampireAttack.OnBiteDamageComplete`
  (params (OtherCombatComponent :type "CombatComponent Object Reference"))
  (`self.ServerBiteDamgeComplete` OtherCombatComponent)
  (`CameraShakeSourceComponent.StartCameraShake` :`self` (`self.CameraShakeSource`) :`InCameraShake` "/Game/Frazier/Creative/Player/BP_BiteCameraShake.BP_BiteCameraShake_C"))

(event `ServerBiteDamgeComplete`
  (params (NewParam :type "CombatComponent Object Reference")))

(event `PressE`
  (`WidgetInteractionComponent.PressPointerKey` (`self.WidgetInteraction`) "LeftMouseButton"))

(event `Key|E`
  (params (Key :type "Key Structure"))
  (:`Pressed`
    (`self.PressE`))
  (:`Released`
    (`self.RelE`)))

(event `RelE`
  (`WidgetInteractionComponent.ReleasePointerKey` (`self.WidgetInteraction`) "LeftMouseButton"))

(event `self.ItemStack.OnUpdateCurrentItems`
  (`self.ClientUpdateItemDisplay`))

(event `ClientUpdateItemDisplay`
  (bind _itemdisplay (`self.ItemDisplay`))
  (bind _itemgridpanel (`/Game/Frazier/Creative/Items/WBP_ItemDisplay.ItemGridPanel` _itemdisplay))
  (`/Engine/EditorBlueprintResources/StandardMacros.IsValid` _itemdisplay
    (:`Is Valid`
      (if (`PanelWidget.HasAnyChildren` _itemgridpanel)
        (`PanelWidget.ClearChildren` _itemgridpanel))
      (for (_array_element _array_index) (`self.K2_GetComponentsByClass` "/Script/SteamCompany.ItemEffectComponent")
        (bind _asplayer_controller (cast `PlayerController` (`self.GetController` self)))
        (bind _returnvalue (`|CreateWidget` "/Game/Frazier/Creative/Items/WBP_Item.WBP_Item_C" _asplayer_controller (`ItemEffectComponent.ItemCount` _array_element)))
        (set `/Game/Frazier/Creative/Items/WBP_Item.ItemImageBrush` (make `SlateBrush` "Image" "NoTile" "NoMirror" (struct :`X` 32.0 :`Y` 32.0) (struct) (struct :`SpecifiedColor` (struct :`R` 1.0 :`G` 1.0 :`B` 1.0 :`A` 1.0) :`ColorUseRule` "UseColor_Specified") (struct :`CornerRadii` (struct :`W` 1.0) :`Color` (struct :`SpecifiedColor` (struct) :`ColorUseRule` "UseColor_Specified") :`RoundingType` "HalfHeightRadius") (`ItemEffectComponent.ItemIconTexture` _array_element)) _returnvalue)
        (bind _returnvalue_2 (`PanelWidget.AddChild` (`/Game/Frazier/Creative/Items/WBP_ItemDisplay.ItemGridPanel` (`self.ItemDisplay`)) _returnvalue))
        (bind _asgrid_slot (cast `GridSlot` _returnvalue_2))
        (`GridSlot.SetRow` _asgrid_slot (mod _array_index 3))
        (`GridSlot.SetColumn` _asgrid_slot (/ _array_index 3))))))

(event `self.Combat.OnActorDead`
  (`self.Dead_Server`))

(event `Dead_Server`
  (bind _returnvalue (`|SpawnActorFromClass` "/Game/Frazier/Creative/BP_PlayerSpectator.BP_PlayerSpectator_C" (`self.GetTransform`) "Undefined" "MultiplyWithRoot" null null))
  (bind _asplayer_controller (cast `PlayerController` (`self.GetController` self)))
  (`/Engine/EditorBlueprintResources/StandardMacros.IsValid` _returnvalue
    (:`Is Valid`
      (`Controller.Possess` _asplayer_controller _returnvalue)
      (`self.K2_DestroyActor`))))

(event `ChangeDialogText_Client`
  (params (InString :type String))
  (bind _dialogdisplay (`self.DialogDisplay`))
  (`/Engine/EditorBlueprintResources/StandardMacros.IsValid` _dialogdisplay
    (:`Is Valid`
      (set `/Game/Frazier/Creative/Lair/WBP_Dialog.DialogText` (`KismetTextLibrary.Conv_StringToText` InString) _dialogdisplay)
      (`Widget.SetVisibility` _dialogdisplay "Visible")
      (`GameplayStatics.PlaySound2D` "/Game/Frazier/Creative/Sounds/laugh1.laugh1" 1.0 1.0 0.0 null null))))

(event `self.DialogSystem.OnChangeDialogText`
  (params (DialogText :type String))
  (`self.ChangeDialogText_Client` DialogText))

(event `EndDialogSystem_Client`
  (bind _dialogdisplay (`self.DialogDisplay`))
  (`/Engine/EditorBlueprintResources/StandardMacros.IsValid` _dialogdisplay
    (:`Is Valid`
      (`Widget.SetVisibility` _dialogdisplay "Hidden"))))

(event `self.DialogSystem.OnEndDialog`
  (`self.EndDialogSystem_Client`))

(event `ShopChange_Client`
  (params (Array :type "Array of ItemEffectComponent Class Reference"))
  (`Widget.SetVisibility` (`self.ShopDisplay`) "Visible")
  (for _array_element Array
    (bind _asplayer_controller (cast `PlayerController` (`self.GetController`)))
    (bind (_itemcount _itemicontexture _itemname) (defaults `Object` _array_element))
    (bind _returnvalue (`|CreateWidget` "/Game/Frazier/Creative/Lair/WBP_ItemCard.WBP_ItemCard_C" _asplayer_controller (`KismetTextLibrary.Conv_StringToText` _itemname) (make `SlateBrush` "Image" "NoTile" "NoMirror" (struct :`X` 32.0 :`Y` 32.0) (struct) (struct :`SpecifiedColor` (struct :`R` 1.0 :`G` 1.0 :`B` 1.0 :`A` 1.0) :`ColorUseRule` "UseColor_Specified") (struct :`CornerRadii` (struct :`W` 1.0) :`Color` (struct :`SpecifiedColor` (struct) :`ColorUseRule` "UseColor_Specified") :`RoundingType` "HalfHeightRadius") _itemicontexture) _array_element))
    (bind _returnvalue_2 (`PanelWidget.AddChild` (`/Game/Frazier/Creative/Lair/WBP_Shop.ItemCardHorizontalBox` (`self.ShopDisplay`)) _returnvalue))
    (bind _ashorizontal_box_slot (cast `HorizontalBoxSlot` _returnvalue_2))
    (`HorizontalBoxSlot.SetSize` _ashorizontal_box_slot (make `SlateChildSize` 1.0))
    (`HorizontalBoxSlot.SetPadding` _ashorizontal_box_slot (make `Margin` 10.0 0.0 10.0))
    (`HorizontalBoxSlot.SetVerticalAlignment` _ashorizontal_box_slot "VAlign_Center")
    (`HorizontalBoxSlot.SetHorizontalAlignment` _ashorizontal_box_slot "HAlign_Center")
    (`MovementComponent.StopMovementImmediately` (`self.CharacterMovement`)))
  (`GameplayStatics.PlaySound2D` "/Game/Frazier/Creative/Sounds/laugh1.laugh1" 1.0 1.5 0.0 null null))

(event `self.ShopSystem.OnShopChange`
  (params (ItemOptions :type "Array of ItemEffectComponent Class Reference (by ref)"))
  (`self.ShopChange_Client` ItemOptions))

(event `EndDialogShop_Client`
  (`Widget.SetVisibility` (`self.ShopDisplay`) "Collapsed"))

(event `self.ShopSystem.OnEndDialog`
  (`self.EndDialogShop_Client`))

(event `self.DashAbility.OnCooldownBegin`
  (params (DashCooldown :type "Float (single-precision)"))
  (bind _ns_speedlines (`self.NS_SpeedLines`))
  (bind _abilitydisplay (`self.AbilityDisplay`))
  (bind _dash (`/Game/Frazier/Creative/Player/WBP_AbilityDisplay.Dash` _abilitydisplay))
  (`|ExecutionSequence`
    (:`then_0`
      (`GameplayStatics.PlaySound2D` "/Game/Frazier/Creative/AI/SpearKnight/whoosh-6316.whoosh-6316" 1.0 1.0 0.0 null null)
      (`ActorComponent.Activate` _ns_speedlines false)
      (`KismetSystemLibrary.Delay` (`DashAbilityComponent.InvincibilityTime` (`self.DashAbility`)))
      (`ActorComponent.Deactivate` _ns_speedlines))
    (:`then_1`
      (`/Engine/EditorBlueprintResources/StandardMacros.IsValid` _abilitydisplay
        (:`Is Valid`
          (`UserWidget.PlayAnimation` _dash (`/Game/Frazier/Creative/Player/WBP_BiteAbilityUI.Cooldown` _dash) 0.0 1 "Forward" (/ 1.0 DashCooldown) true))))))

(event `self.SpearThrow.OnCooldownBegin`
  (params (BiteCooldown :type "Float (single-precision)"))
  (bind _abilitydisplay (`self.AbilityDisplay`))
  (bind _spit (`/Game/Frazier/Creative/Player/WBP_AbilityDisplay.Spit` _abilitydisplay))
  (`GameplayStatics.PlaySoundAtLocation` "/Game/Frazier/Creative/Player/whip-123738.whip-123738" (0.0 0.0 0.0) (struct) 1.0 1.0 0.0 null null null null)
  (`/Engine/EditorBlueprintResources/StandardMacros.IsValid` _abilitydisplay
    (:`Is Valid`
      (`UserWidget.PlayAnimation` _spit (`/Game/Frazier/Creative/Player/WBP_BiteAbilityUI.Cooldown` _spit) 0.0 1 "Forward" (/ 1.0 BiteCooldown) true))))

(fn `UserConstructionScript`)