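; PC_Fight is a controller Blueprint that sets up the start of a fight level called "Earth Realm".
; BeginPlay plays pitched-down music, shows a level intro widget with movement input briefly locked, and adds statue, boss and portal objectives to the pawn's ObjectiveSystemComponent.
; Its Server event waits, then moves every character whose CombatComponent flags it as a player to just above the first BP_EnemySpawnNode found.
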(event `self.ReceiveBeginPlay`
  (bind _returnvalue (`self.GetComponentByClass` (`self.K2_GetPawn` self) "/Script/SteamCompany.ObjectiveSystemComponent"))
  (bind _currentobjectives (`ObjectiveSystemComponent.CurrentObjectives` _returnvalue))
  (`self.Server`)
  (`|ExecutionSequence`
    (:`then_0`
      (`KismetSystemLibrary.Delay` 0.01)
      (`GameplayStatics.PlaySound2D` "/Game/Frazier/Creative/Sounds/kingdom.kingdom" 0.4 0.6 0.0 null null)
      (bind _asplayer_controller (cast `PlayerController` (`Pawn.GetController` (`self.K2_GetPawn`))))
      (`|ExecutionSequence`
        (:`then_1`
          (bind _returnvalue_2 (`|CreateWidget` "/Game/Frazier/Creative/Player/Widgets/WBP_LevelEnter.WBP_LevelEnter_C" _asplayer_controller "Earth Realm" (make `SlateColor` (`self.Color Specified Color`))))
          (`/Engine/EditorBlueprintResources/StandardMacros.IsValid` _returnvalue_2
            (:`Is Valid`
              (`UserWidget.AddToViewport` _returnvalue_2 0)
              (`self.SetIgnoreMoveInput` true)
              (`KismetSystemLibrary.Delay` 3.0)
              (`self.SetIgnoreMoveInput` false))))))
    (:`then_1`
      (`/Engine/EditorBlueprintResources/StandardMacros.IsValid` _returnvalue
        (:`Is Valid`
          (`KismetArrayLibrary.Array_Add` _currentobjectives "DestroySacredStatues")
          (`KismetArrayLibrary.Array_Add` _currentobjectives "KillBoss")
          (`KismetArrayLibrary.Array_Add` _currentobjectives "EnterPortal"))))))

(event `Server`
  (`KismetSystemLibrary.Delay` 3.0)
  (bind _outactors (`GameplayStatics.GetAllActorsOfClass` "/Script/Engine.Character"))
  (for _array_element _outactors
    (bind _returnvalue (`self.GetComponentByClass` _array_element "/Script/SteamCompany.CombatComponent"))
    (`/Engine/EditorBlueprintResources/StandardMacros.IsValid` _returnvalue
      (:`Is Valid`
        (if (`CombatComponent.bIsPlayer` _returnvalue)
          (bind _outactors_2 (`GameplayStatics.GetAllActorsOfClass` "/Game/Frazier/Creative/AI/BP_EnemySpawnNode.BP_EnemySpawnNode_C"))
          (bind _output (`|GetArrayItem` _outactors_2))
          (`/Engine/EditorBlueprintResources/StandardMacros.IsValid` _output
            (:`Is Valid`
              (bind (_returnvalue_x _returnvalue_y _returnvalue_z) (`KismetMathLibrary.BreakVector` (`self.K2_GetActorLocation` _output)))
              (`self.K2_SetActorLocation` _array_element (`KismetMathLibrary.MakeVector` _returnvalue_x _returnvalue_y (+ _returnvalue_z 200.0)) false false))))))))

(fn `UserConstructionScript`)