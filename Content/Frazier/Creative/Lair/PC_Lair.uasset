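; Player controller for the Jester Gods Lair level that runs the level intro and hands out starting objectives.
; BeginPlay calls a Client event which, after a tiny delay, plays a low-pitched piano sound, shows the WBP_LevelEnter title widget and ignores move input for three seconds.
; Without waiting for those delays, it adds the talk-to-Jester-God and shop objectives to the pawn's ObjectiveSystemComponent.
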(event `self.ReceiveBeginPlay`
  (`self.Client`))

(event `Client`
  (bind _returnvalue (`self.GetComponentByClass` (`self.K2_GetPawn` self) "/Script/SteamCompany.ObjectiveSystemComponent"))
  (bind _currentobjectives (`ObjectiveSystemComponent.CurrentObjectives` _returnvalue))
  (`|ExecutionSequence`
    (:`then_0`
      (`KismetSystemLibrary.Delay` 0.01)
      (`GameplayStatics.PlaySound2D` "/Game/Frazier/Creative/Sounds/piano.piano" 0.4 0.6 0.0 null null)
      (`|ExecutionSequence`
        (:`then_1`
          (bind _returnvalue_2 (`|CreateWidget` "/Game/Frazier/Creative/Player/WBP_LevelEnter.WBP_LevelEnter_C" self "Jester Gods Lair" (make `SlateColor` (`self.Color Specified Color`))))
          (`/Engine/EditorBlueprintResources/StandardMacros.IsValid` _returnvalue_2
            (:`Is Valid`
              (`UserWidget.AddToViewport` _returnvalue_2 0)
              (`self.SetIgnoreMoveInput` true)
              (`KismetSystemLibrary.Delay` 3.0)
              (`self.SetIgnoreMoveInput` false))))))
    (:`then_1`
      (`/Engine/EditorBlueprintResources/StandardMacros.IsValid` _returnvalue
        (:`Is Valid`
          (`KismetArrayLibrary.Array_Add` _currentobjectives "TalkJesterGod")
          (`KismetArrayLibrary.Array_Add` _currentobjectives "TalkShop"))))))

(fn `UserConstructionScript`)