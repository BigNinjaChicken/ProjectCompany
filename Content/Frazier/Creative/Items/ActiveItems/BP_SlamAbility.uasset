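; BP_SlamAbility is a slam active-item ability that adds audio and visual feedback to events on its owning actor.
; On BeginPlay it binds handlers to the inherited cooldown-begin and slam-complete delegates; the slam logic itself is not in this graph.
; Cooldown start plays an eject sound at the owner, while slam completion plays an underwater explosion sound and spawns an enlarged burst particle below the owner.
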(event `self.ReceiveBeginPlay`
  (`|ExecutionSequence`
    (:`then_0`
      (add `self.OnCooldownBegin` (delegate `OnCooldownBegin_Event`)))
    (:`then_1`
      (add `self.OnSlamComplete` (delegate `OnSlamComplete_Event`)))))

(event `OnCooldownBegin_Event` :!signature `self.OnCooldownBegin`
  (params (BiteCooldown :type "Float (single-precision)"))
  (`GameplayStatics.PlaySoundAtLocation` "/Engine/EditorSounds/GamePreview/EjectFromPlayer.EjectFromPlayer" (`Actor.K2_GetActorLocation` (`self.GetOwner`)) (struct) 1.0 1.0 0.0 null null null null))

(event `OnSlamComplete_Event`
  (bind _returnvalue (`self.GetOwner`))
  (bind (_returnvalue_x _returnvalue_y _returnvalue_z) (`KismetMathLibrary.BreakVector` (`Actor.K2_GetActorLocation` _returnvalue)))
  (`GameplayStatics.PlaySoundAtLocation` "/Game/Frazier/Creative/Sounds/large-underwater-explosion-190270.large-underwater-explosion-190270" (`Actor.K2_GetActorLocation` _returnvalue) (struct) 1.0 1.0 0.0 null null null null)
  (`GameplayStatics.SpawnEmitterAtLocation` "/Game/InfinityBladeEffects/Effects/FX_Skill_RockBurst/P_RBurst_Default_Burst_SinkH_01.P_RBurst_Default_Burst_SinkH_01" (`KismetMathLibrary.MakeVector` _returnvalue_x _returnvalue_y (- _returnvalue_z 100.0)) (struct) (3.0 3.0 3.0)))