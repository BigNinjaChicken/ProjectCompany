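; Spear Knight AI enemy character that reacts to its Combat and SpearThrow component events.
; Damage, spear throws and death route to Multi events for cosmetic feedback: sounds, plus blood bursts on hit and death.
; Death plays its effects once, stops the AI brain, disables movement and turns the capsule into a physics body launched backward.
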(event `Dead_Multi`
  (`NiagaraFunctionLibrary.SpawnSystemAtLocation` "/Game/Artin/Particles/NS_BloodBurst.NS_BloodBurst" (`self.K2_GetActorLocation`))
  (`GameplayStatics.PlaySoundAtLocation` "/Game/Frazier/Creative/Sounds/laugh2.laugh2" (`self.K2_GetActorLocation`) (struct) 1.0 1.0 0.0 null null null null))

(event `self.Combat.OnActorDead`
  (`|ExecutionSequence`
    (:`then_0`
      (`/Engine/EditorBlueprintResources/StandardMacros.DoOnce` false
        (:`Completed`
          (`self.Dead_Multi`))))
    (:`then_1`
      (`PrimitiveComponent.SetSimulatePhysics` (`self.CapsuleComponent`) true)
      (`CharacterMovementComponent.DisableMovement` (`self.CharacterMovement`))
      (`BrainComponent.StopLogic` (`AIController.BrainComponent` (`AIBlueprintHelperLibrary.GetAIController` self)) "I said so")
      (`PrimitiveComponent.AddImpulse` (`self.CapsuleComponent`) (* (`KismetMathLibrary.NegateVector` (`SceneComponent.GetForwardVector` (`self.CapsuleComponent`))) 800.0) "None" true))))

(event `self.SpearThrow.OnSpearThrown`
  (params (Spear :type "SpearProjectileActor Object Reference"))
  (`self.SpearThrown_Multi`))

(event `SpearThrown_Multi`
  (`GameplayStatics.PlaySoundAtLocation` "/Game/Frazier/Creative/AI/SpearKnight/axe-slash-1-106748.axe-slash-1-106748" (`self.K2_GetActorLocation`) (struct) 1.0 1.0 0.0 null null null null))

(event `self.Combat.OnTakeDamageComplete`
  (`self.TakeDamge_Multi`))

(event `TakeDamge_Multi`
  (`NiagaraFunctionLibrary.SpawnSystemAttached` "/Game/Artin/Particles/NS_BloodBurst.NS_BloodBurst" (`self.Mesh`) "None" (0.0 0.0 0.0) (struct) "KeepRelativeOffset" true)
  (`GameplayStatics.PlaySoundAtLocation` "/Game/Frazier/Creative/AI/NPC/homemadeoof-47509.homemadeoof-47509" (`self.K2_GetActorLocation`) (struct) 1.0 1.0 0.0 null null null null))

(fn `UserConstructionScript`)