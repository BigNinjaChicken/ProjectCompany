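; BP_PlayerSpectator is the player spectator Blueprint, which shows a spectating UI and prompts a game-over check when possessed.
; On BeginPlay it retries every half second until its controller is a PlayerController, then creates WBP_Spectating for that player and adds it to the viewport.
; On possession it calls its Server event, which casts the game mode to GM_MainGame and runs CheckGameOver.
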(event `self.ReceivePossessed`
  (params (NewController :type "Controller Object Reference"))
  (`self.Server`))

(event `self.ReceiveBeginPlay`
  (bind _asplayer_controller (cast `PlayerController` (`self.GetController`) :!label _label)
    (:`then`
      (bind _returnvalue (`|CreateWidget` "/Game/Frazier/Creative/Player/WBP_Spectating.WBP_Spectating_C" _asplayer_controller))
      (`UserWidget.AddToViewport` _returnvalue 0))
    (:`CastFailed`
      (`KismetSystemLibrary.Delay` 0.5)
      (goto _label))))

(event `Server`
  (bind _asgm_main_game (cast `/Game/Frazier/Creative/GM_MainGame` (`GameplayStatics.GetGameMode`)))
  (`/Game/Frazier/Creative/GM_MainGame.CheckGameOver` _asgm_main_game))

(fn `UserConstructionScript`)