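; Vampire player Blueprint that adds HUD and hit feedback to the bite ability of its VampireAttack component.
; BeginPlay creates the ability display widget for its first-person player controller.
; Bite cooldown events play the UI cooldown animation, scaled to match the cooldown duration.
; Completed bite damage routes through a multicast event that starts a camera shake and attaches a Niagara blood burst to the victim.
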(event `self.ReceiveBeginPlay`
  (bind _asbp_first_person_player_controller (cast `/Game/FirstPerson/Blueprints/BP_FirstPersonPlayerController` (`self.GetController` self)))
  (bind _returnvalue (`|CreateWidget` "/Game/Frazier/Creative/WBP_AbilityDisplay.WBP_AbilityDisplay_C" _asbp_first_person_player_controller))
  (bind _output_get (set `self.AbilityDisplay` _returnvalue))
  (`UserWidget.AddToViewport` _output_get 0))

(event `self.VampireAttack.OnBiteCooldownBegin`
  (params (BiteCooldown :type "Float (single-precision)"))
  (bind _wbp_biteabilityui (`/Game/Frazier/Creative/WBP_AbilityDisplay.WBP_BiteAbilityUI` (`self.AbilityDisplay`)))
  (`UserWidget.PlayAnimation` _wbp_biteabilityui (`/Game/Frazier/Creative/WBP_BiteAbilityUI.Cooldown` _wbp_biteabilityui) 0.0 1 "Forward" (/ 1.0 BiteCooldown) true))

(event `self.VampireAttack.OnBiteDamageComplete`
  (params (OtherCombatComponent :type "CombatComponent Object Reference"))
  (`self.MulticastBiteDamageComplete` OtherCombatComponent))

(event `MulticastBiteDamageComplete`
  (params (`Other Combat Component` :type "CombatComponent Object Reference"))
  (`/Engine/EditorBlueprintResources/StandardMacros.IsValid` `Other Combat Component`
    (:`Is Valid`
      (`CameraShakeSourceComponent.StartCameraShake` :`self` (`self.CameraShakeSource`) :`InCameraShake` "/Game/Frazier/Creative/BP_BiteCameraShake.BP_BiteCameraShake_C")
      (`NiagaraFunctionLibrary.SpawnSystemAttached` "/Game/Artin/Particles/NS_BloodBurst.NS_BloodBurst" (`Actor.RootComponent` (`ActorComponent.GetOwner` `Other Combat Component`)) "None" (0.0 0.0 0.0) (struct) "KeepRelativeOffset" true))))

(fn `UserConstructionScript`)