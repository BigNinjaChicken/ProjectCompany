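; Base enemy Blueprint that chases the player and plays a melee-range attack animation on reaching them.
; BeginPlay starts ChasePlayer, which runs AI MoveTo toward player 0; on success, Attack plays a montage on the mesh, then the chase repeats after a short delay.
; Only the success output continues the loop, so a failed move ends the chase, and Attack contains no damage logic.
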(event `self.ReceiveBeginPlay`
  (`self.ChasePlayer`))

(event `ChasePlayer`
  ;[1 1 1] Chase
  (`|AIMoveTo` self (0.0 0.0 0.0) (`GameplayStatics.GetPlayerCharacter` 0) 150.0
    (:`OnSuccess`
      (`self.Attack`)
      (`KismetSystemLibrary.Delay` 2.0)
      (`self.ChasePlayer`))))

(event `Attack`
  (`|PlayMontage` (`self.Mesh`) "/Game/Artin/Animation/Chuck_Sequence_Montage.Chuck_Sequence_Montage"))

(fn `UserConstructionScript`)