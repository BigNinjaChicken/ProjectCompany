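; BP_HolyGhost is an AI ghost character that reacts to damage and death reported by its Combat component.
; Surviving hits knock it backward along its facing axis and play a breath sound through a Multi event.
; Death triggers a one-time blood burst and laughing sound, then stops movement and AI logic and launches the physics-simulated capsule backward.
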(event `Dead_Multi`
  (`NiagaraFunctionLibrary.SpawnSystemAtLocation` "/Game/Artin/Particles/NS_BloodBurst.NS_BloodBurst" (`self.K2_GetActorLocation`))
  (`GameplayStatics.PlaySoundAtLocation` "/Game/Ethan/Sound/laughing-ghost-horror-sounds.laughing-ghost-horror-sounds" (`self.K2_GetActorLocation`) (struct) 1.0 1.0 0.0 null null null null))

(event `self.Combat.OnActorDead`
  (`|ExecutionSequence`
    (:`then_0`
      (`/Engine/EditorBlueprintResources/StandardMacros.DoOnce` false
        (:`Completed`
          (`self.Dead_Multi`))))
    (:`then_1`
      (`PrimitiveComponent.SetSimulatePhysics` (`self.CapsuleComponent`) true)
      (`CharacterMovementComponent.DisableMovement` (`self.CharacterMovement`))
      (`BrainComponent.StopLogic` (`AIController.BrainComponent` (`AIBlueprintHelperLibrary.GetAIController` self)) "I said so")
      (`PrimitiveComponent.AddImpulse` (`self.CapsuleComponent`) (* (`KismetMathLibrary.NegateVector` (`SceneComponent.GetForwardVector` (`self.CapsuleComponent`))) 800.0) "None" true))))

(event `self.Combat.OnTakeDamageComplete`
  (if (> (`CombatComponent.Health` (`self.Combat`)) 0.0)
    (`CharacterMovementComponent.AddImpulse` (`self.CharacterMovement`) (* (`KismetMathLibrary.NegateVector` (`SceneComponent.GetForwardVector` (`self.CapsuleComponent`))) 3000.0) true)
    (`self.DamageComplete_Multi`)))

(event `DamageComplete_Multi`
  (`GameplayStatics.PlaySoundAtLocation` "/Game/Ethan/Sound/giant-breath.giant-breath" (`self.K2_GetActorLocation`) (struct) 1.0 1.0 0.0 null null null null))

(fn `UserConstructionScript`)