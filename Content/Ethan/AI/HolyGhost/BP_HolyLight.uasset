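; BP_HolyLight is a timed Holy Ghost area hazard that damages the vampire player with a column of holy light.
; On spawn it plays a choir sound and widens the light mesh from zero over GrowthTime, then switches to a damage material with a thunder sound.
; Once armed, Tick applies fixed damage at DamageRate intervals while overlap events flag the player inside.
; The actor destroys itself after GrowthTime plus LingerTime.
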(event `self.ReceiveActorEndOverlap`
  (params (OtherActor :type "Actor Object Reference"))
  (bind _returnvalue (`self.GetComponentByClass` OtherActor "/Script/SteamCompany.CombatComponent"))
  (`/Engine/EditorBlueprintResources/StandardMacros.IsValid` _returnvalue
    (:`Is Valid`
      (if (`CombatComponent.bIsPlayer` _returnvalue)
        (set `self.touchingPlayer` false)))))

(event `self.ReceiveBeginPlay`
  (`GameplayStatics.PlaySoundAtLocation` "/Game/Ethan/Sound/short-choir.short-choir" (`self.K2_GetActorLocation`) (struct) 1.0 1.0 0.0 null null null null)
  (`SceneComponent.SetRelativeScale3D` (`self.LightMesh`) (0.0 0.0 1.0))
  (`KismetSystemLibrary.Delay` (+ (`self.lingerTime`) (`self.GrowthTime`)))
  (`self.K2_DestroyActor`))

(event `self.ReceiveActorBeginOverlap`
  (params (OtherActor :type "Actor Object Reference"))
  (bind _returnvalue (`self.GetComponentByClass` OtherActor "/Script/SteamCompany.CombatComponent"))
  (set `self.Other Actor` OtherActor)
  (`/Engine/EditorBlueprintResources/StandardMacros.IsValid` _returnvalue
    (:`Is Valid`
      (if (`CombatComponent.bIsPlayer` _returnvalue)
        (set `self.touchingPlayer` true)))))

(event `self.ReceiveTick`
  (params (DeltaSeconds :type "Float (single-precision)"))
  (set `self.Delta Seconds` DeltaSeconds)
  (`self.Grow`)
  (`self.DamagePlayer`)
  (`self.DamageTimer`))

(event `DamagePlayer`
  (if (`self.touchingPlayer`)
    (if (`self.doDamage`)
      (if (>= (`self.damageTime`) (`self.damageRate`))
        (set `self.damageTime` 0.0)
        (bind _asbp_vampire_player (cast `/Game/Frazier/Creative/Player/BP_VampirePlayer` (`self.Other Actor`)))
        (`CombatComponent.ServerTakeDamage` (`/Game/Frazier/Creative/Player/BP_VampirePlayer.Combat` _asbp_vampire_player) 15.0)))))

(event `Grow`
  (bind _lightmesh (`self.LightMesh`))
  (bind (_relativescale3d_x _relativescale3d_y) (`KismetMathLibrary.BreakVector` (`SceneComponent.RelativeScale3D` _lightmesh)))
  (bind _returnvalue (* (/ (`self.MaxGrowth`) (`self.GrowthTime`)) (`self.Delta Seconds`)))
  (if (`self.doDamage`)
    _
    (elif (> (`self.MaxGrowth`) _relativescale3d_x)
      (`SceneComponent.SetRelativeScale3D` _lightmesh (`KismetMathLibrary.MakeVector` (+ _relativescale3d_x _returnvalue) (+ _relativescale3d_y _returnvalue) 1.0))
      (else
        (`PrimitiveComponent.SetMaterial` (`self.LightMesh`) 0 "/Game/Ethan/Materials/MT_Light_Inst_Damage.MT_Light_Inst_Damage")
        (set `self.doDamage` true)
        (`GameplayStatics.PlaySoundAtLocation` "/Game/Ethan/Sound/thunder-edit.thunder-edit" (`self.K2_GetActorLocation`) (struct) 1.0 1.0 0.0 null null null null)))))

(event `DamageTimer`
  (set `self.damageTime` (+ (`self.damageTime`) (`self.Delta Seconds`))))

(fn `UserConstructionScript`)