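; Player character for the multiplayer vampire, handling its HUD, proximity voice chat and bite feedback.
; BeginPlay creates ability, health and item widgets and registers a VOIP talker, retrying until PlayerState is valid; V is push-to-talk.
; Tick refreshes health from Combat, while ItemStack updates rebuild the item grid from ItemEffectComponents.
; VampireAttack events drive the cooldown animation, camera shake and server-to-multicast blood burst; E clicks through WidgetInteraction.
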(event `Key|N`
  (params (Key :type "Key Structure"))
  (:`Pressed`
    (`KismetSystemLibrary.ExecuteConsoleCommand` "stat net" null)))

(event `Key|V`
  (params (Key :type "Key Structure"))
  (:`Pressed`
    (`KismetSystemLibrary.ExecuteConsoleCommand` "ToggleSpeaking 1" null))
  (:`Released`
    (`KismetSystemLibrary.ExecuteConsoleCommand` "ToggleSpeaking 0" null)))

(event `self.ReceiveBeginPlay`
  (bind _playerstate (`self.PlayerState`))
  (bind _widgetinteraction (`self.WidgetInteraction`))
  (bind _returnvalue (`GameplayStatics.GetPlayerControllerID` (`self.GetLocalViewingPlayerController`)))
  (`|ExecutionSequence`
    (:`then_0`
      (bind _returnvalue_2 (`AddComponent|NODE_AddVOIPTalker-2`))
      (bind _output_get (set `self.VOIPTalker` _returnvalue_2))
      (`/Engine/EditorBlueprintResources/StandardMacros.IsValid` _playerstate :!label _label
        (:`Is Valid`
          (`VOIPTalker.RegisterWithPlayerState` _output_get _playerstate)
          (`VOIPStatics.SetMicThreshold` -1.0)
          (set `VOIPTalker.Settings` (make `VoiceSettings` (`self.FirstPersonCameraComponent`) "/Game/Frazier/Creative/Player/VC_SoundAttenuation.VC_SoundAttenuation") (`self.VOIPTalker`)))
        (:`Is Not Valid`
          (`KismetSystemLibrary.Delay` 1.0)
          (goto _label))))
    (:`then_1`
      (bind _asbp_first_person_player_controller (cast `/Game/FirstPerson/Blueprints/BP_FirstPersonPlayerController` (`self.GetController` self)))
      (`|ExecutionSequence`
        (:`then_0`
          (bind _returnvalue_3 (`|CreateWidget` "/Game/Frazier/Creative/Player/WBP_AbilityDisplay.WBP_AbilityDisplay_C" _asbp_first_person_player_controller))
          (bind _output_get_2 (set `self.AbilityDisplay` _returnvalue_3))
          (`UserWidget.AddToViewport` _output_get_2 0))
        (:`then_1`
          (bind _returnvalue_4 (`|CreateWidget` "/Game/Frazier/Creative/Player/WBP_Health.WBP_Health_C" _asbp_first_person_player_controller))
          (bind _output_get_3 (set `self.HealthDisplay` _returnvalue_4))
          (`UserWidget.AddToViewport` _output_get_3 0)
          (`self.ClientUpdateHealthDisplay`))
        (:`then_2`
          (bind _returnvalue_5 (`|CreateWidget` "/Game/Frazier/Creative/Items/WBP_ItemDisplay.WBP_ItemDisplay_C" _asbp_first_person_player_controller))
          (bind _output_get_4 (set `self.ItemDisplay` _returnvalue_5))
          (`UserWidget.AddToViewport` _output_get_4 0))))
    (:`then_2`
      (set `WidgetInteractionComponent.PointerIndex` _returnvalue _widgetinteraction)
      (set `WidgetInteractionComponent.PointerIndex` _returnvalue _widgetinteraction))))

(event `self.ReceiveTick`
  (params (DeltaSeconds :type "Float (single-precision)"))
  (`self.ClientUpdateHealthDisplay`))

(event `ClientUpdateHealthDisplay`
  (bind _combat (`self.Combat`))
  (bind _healthdisplay (`self.HealthDisplay`))
  (`/Engine/EditorBlueprintResources/StandardMacros.IsValid` _healthdisplay
    (:`Is Valid`
      (`/Engine/EditorBlueprintResources/StandardMacros.IsValid` _combat
        (:`Is Valid`
          (set `/Game/Frazier/Creative/Player/WBP_Health.HealthPercent` (`KismetMathLibrary.MapRangeClamped` (`CombatComponent.Health` _combat) 0.0 (`CombatComponent.MaxHealth` _combat) 0.0 1.0) _healthdisplay))))))

(event `self.VampireAttack.OnBiteCooldownBegin`
  (params (BiteCooldown :type "Float (single-precision)"))
  (bind _abilitydisplay (`self.AbilityDisplay`))
  (bind _wbp_biteabilityui (`/Game/Frazier/Creative/Player/WBP_AbilityDisplay.WBP_BiteAbilityUI` _abilitydisplay))
  (`/Engine/EditorBlueprintResources/StandardMacros.IsValid` _abilitydisplay
    (:`Is Valid`
      (`UserWidget.PlayAnimation` _wbp_biteabilityui (`/Game/Frazier/Creative/Player/WBP_BiteAbilityUI.Cooldown` _wbp_biteabilityui) 0.0 1 "Forward" (/ 1.0 BiteCooldown) true))))

(event `self.VampireAttack.OnBiteDamageComplete`
  (params (OtherCombatComponent :type "CombatComponent Object Reference"))
  (`self.ServerBiteDamgeComplete` OtherCombatComponent)
  (`CameraShakeSourceComponent.StartCameraShake` :`self` (`self.CameraShakeSource`) :`InCameraShake` "/Game/Frazier/Creative/Player/BP_BiteCameraShake.BP_BiteCameraShake_C"))

(event `ServerBiteDamgeComplete`
  (params (NewParam :type "CombatComponent Object Reference"))
  (`self.MulticastBiteDamageComplete` NewParam))

(event `MulticastBiteDamageComplete`
  (params (`Other Combat Component` :type "CombatComponent Object Reference"))
  (`/Engine/EditorBlueprintResources/StandardMacros.IsValid` `Other Combat Component`
    (:`Is Valid`
      (`NiagaraFunctionLibrary.SpawnSystemAttached` "/Game/Artin/Particles/NS_BloodBurst.NS_BloodBurst" (`Actor.RootComponent` (`ActorComponent.GetOwner` `Other Combat Component`)) "None" (0.0 0.0 0.0) (struct) "KeepRelativeOffset" true))))

(event `Key|E`
  (params (Key :type "Key Structure"))
  (bind _widgetinteraction (`self.WidgetInteraction`))
  (:`Pressed`
    (`WidgetInteractionComponent.PressPointerKey` _widgetinteraction "LeftMouseButton"))
  (:`Released`
    (`WidgetInteractionComponent.ReleasePointerKey` _widgetinteraction "LeftMouseButton")))

(event `self.ItemStack.OnUpdateCurrentItems`
  (`self.ClientUpdateItemDisplay`))

(event `ClientUpdateItemDisplay`
  (bind _itemdisplay (`self.ItemDisplay`))
  (bind _itemgridpanel (`/Game/Frazier/Creative/Items/WBP_ItemDisplay.ItemGridPanel` _itemdisplay))
  (`/Engine/EditorBlueprintResources/StandardMacros.IsValid` _itemdisplay
    (:`Is Valid`
      (if (`PanelWidget.HasAnyChildren` _itemgridpanel)
        (`PanelWidget.ClearChildren` _itemgridpanel))
      (for (_array_element _array_index) (`self.K2_GetComponentsByClass` "/Script/SteamCompany.ItemEffectComponent")
        (bind _asbp_first_person_player_controller (cast `/Game/FirstPerson/Blueprints/BP_FirstPersonPlayerController` (`self.GetController` self)))
        (bind _returnvalue (`|CreateWidget` "/Game/Frazier/Creative/Items/WBP_Item.WBP_Item_C" _asbp_first_person_player_controller (`ItemEffectComponent.ItemCount` _array_element)))
        (set `/Game/Frazier/Creative/Items/WBP_Item.ItemImageBrush` (make `SlateBrush` "Image" "NoTile" "NoMirror" (struct :`X` 32.0 :`Y` 32.0) (struct) (struct :`SpecifiedColor` (struct :`R` 1.0 :`G` 1.0 :`B` 1.0 :`A` 1.0) :`ColorUseRule` "UseColor_Specified") (struct :`CornerRadii` (struct :`W` 1.0) :`Color` (struct :`SpecifiedColor` (struct) :`ColorUseRule` "UseColor_Specified") :`RoundingType` "HalfHeightRadius") (`ItemEffectComponent.ItemIconTexture` _array_element)) _returnvalue)
        (bind _returnvalue_2 (`PanelWidget.AddChild` (`/Game/Frazier/Creative/Items/WBP_ItemDisplay.ItemGridPanel` (`self.ItemDisplay`)) _returnvalue))
        (bind _asgrid_slot (cast `GridSlot` _returnvalue_2))
        (`GridSlot.SetRow` _asgrid_slot (mod _array_index 3))
        (`GridSlot.SetColumn` _asgrid_slot (/ _array_index 3))))))

(fn `UserConstructionScript`)