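; BP_MeshTiler is a construction-script tool that lays out copies of a static mesh in a straight row.
; It calls Tile for each index from 1 to TileAmount, adding a static mesh component and assigning NewMesh.
; Each copy is offset by its index times MeshSize, along local X when TilesXorY is true and Y otherwise, so the first sits one step from the origin.
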(fn `Tile`
  (params (MeshIndex :type Integer))
  (bind _tiles_xory_ (`self.Tiles XorY?`))
  (bind _returnvalue (* MeshIndex (`self.MeshSize`)))
  (bind _returnvalue_2 (`AddComponent|NODE_AddStaticMeshComponent-0` :`RelativeTransform` (`KismetMathLibrary.MakeTransform` (`KismetMathLibrary.MakeVector` (`KismetMathLibrary.SelectFloat` _returnvalue 0.0 _tiles_xory_) (`KismetMathLibrary.SelectFloat` 0.0 _returnvalue _tiles_xory_)))))
  (`StaticMeshComponent.SetStaticMesh` _returnvalue_2 (`self.New Mesh`)))

(fn `UserConstructionScript`
  (for _index (range 1 (+ (`self.TileAmount`) 1))
    (`self.Tile` _index)))