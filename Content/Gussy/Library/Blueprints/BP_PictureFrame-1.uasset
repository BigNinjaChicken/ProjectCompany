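; Picture frame prop Blueprint that varies its frame mesh and the painting it displays.
; The construction script assigns a random mesh from NewMesh, then creates a dynamic instance of MI_Painting on material slot 1.
; Its BaseColor texture is either a random entry from PaintingTextureArray or the set PaintingTexture, chosen by IsRandomPainting.
; Random picks are unseeded, so they reroll whenever construction reruns; the event graph is unused.
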(fn `UserConstructionScript`
  (bind _staticmesh (`self.StaticMesh`))
  (`StaticMeshComponent.SetStaticMesh` _staticmesh (`KismetArrayLibrary.Array_Random` (`self.New Mesh`)))
  (bind _returnvalue (`KismetMaterialLibrary.CreateDynamicMaterialInstance` "/Game/Gussy/Library/Materials/MI_Painting.MI_Painting"))
  (`MaterialInstanceDynamic.SetTextureParameterValue` _returnvalue "BaseColor" (select `bool` (`self.isRandomPainting`) :`false` (`self.PaintingTexture`) :`true` (`KismetArrayLibrary.Array_Random` (`self.PaintingTextureArray`))))
  (`PrimitiveComponent.SetMaterial` _staticmesh 1 _returnvalue))