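; BP_WallDecor-Light is a configurable wall decor light that pairs a static mesh with a point light.
; Its construction script gives the mesh a dynamic instance of MI_WallDecorLight1 and applies the shadow, color, radius, intensity and volumetric scattering variables to the light.
; IsOn switches both the emissive glow and the light intensity between their set values and zero.
; It has no active runtime event logic.
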(fn `UserConstructionScript`
  (bind _pointlight (`self.PointLight`))
  (bind _returnvalue (`KismetMaterialLibrary.CreateDynamicMaterialInstance` "/Game/Gussy/Library/Materials/MI_WallDecor-Light-1.MI_WallDecor-Light-1"))
  (`MaterialInstanceDynamic.SetScalarParameterValue` _returnvalue "EmissiveIntensity" (`KismetMathLibrary.SelectFloat` (`self.EmissiveIntensity`) 0.0 (`self.isOn?`)))
  (`PrimitiveComponent.SetMaterial` (`self.StaticMesh`) 0 _returnvalue)
  (`LightComponentBase.SetCastShadows` _pointlight (`self.castsShadows?`))
  (`LightComponent.SetIntensity` _pointlight (`KismetMathLibrary.SelectFloat` (`self.LightIntensity`) 0.0 (`self.isOn?`)))
  (`LightComponent.SetLightColor` _pointlight (`self.Light Color`) true)
  (`LocalLightComponent.SetAttenuationRadius` _pointlight (`self.LightRadius`))
  (`LightComponent.SetVolumetricScatteringIntensity` _pointlight (`self.VolumetricIntensity`)))