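; BP_BookTiler procedurally fills a row of books from static mesh components.
; Tile adds one book per index, spaced along local Y by MeshSize, with random depth offset, width and height.
; Each book gets a random material from MaterialArray on slot 0.
; SpawnBooksInEditor selects whether the row is built in the construction script or on BeginPlay.
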(event `self.ReceiveBeginPlay`
  (if (not (`self.spawnBooksInEditor?`))
    (for _index (range 1 (+ (`self.BookAmount`) 1))
      (`self.Tile` _index))))

(fn `Tile`
  (params (TileAmount :type Integer))
  (bind _returnvalue (`AddComponent|NODE_AddStaticMeshComponent-1` :`RelativeTransform` (`KismetMathLibrary.MakeTransform` (`KismetMathLibrary.MakeVector` (`KismetMathLibrary.RandomFloatInRange` -4.0) (* TileAmount (`self.MeshSize`))) (struct) (`KismetMathLibrary.MakeVector` (`KismetMathLibrary.RandomFloatInRange` 1.0 1.0) (`KismetMathLibrary.RandomFloatInRange` (`self.BookWidthMinimum`) (`self.BookWidthMaximum`)) (`KismetMathLibrary.RandomFloatInRange` (`self.BookHeightMinimum`) (`self.BookHeightMaximum`))))))
  (`PrimitiveComponent.SetMaterial` _returnvalue 0 (`KismetArrayLibrary.Array_Random` (`self.MaterialArray`)))
  (set `self.PreviousMesh` _returnvalue))

(fn `UserConstructionScript`
  (if (`self.spawnBooksInEditor?`)
    (for _index (range 1 (+ (`self.BookAmount`) 1))
      (`self.Tile` _index))))